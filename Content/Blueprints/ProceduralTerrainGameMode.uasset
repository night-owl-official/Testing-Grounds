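; Game mode that builds a procedural terrain strip by spawning a chain of ten BP_Tile actors when play begins.
; The chain continues from the attach point of the last tile found in the world, or starts at the origin when none exist.
; Each spawned tile's attach point becomes the transform for the next, so the tiles link end to end.
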(event EventBeginPlay
  (bind _outactors (Actor|GetAllActorsOfClass "/Game/Blueprints/Tiles/BP_Tile.BP_Tile_C"))
  (if (CallFunction|IsThereAnyTileintheWorld _outactors)
    (Variables|Spawn|SetNextTileTransform (CallFunction|GetLastTile'sTransform _outactors))
    (else
      (Variables|Spawn|SetNextTileTransform (Math|Transform|MakeTransform "0, 0, 0"))))
  (for _index (range 0 9)
    (bind _returnvalue (Game|SpawnActorfromClass "/Game/Blueprints/Tiles/BP_Tile.BP_Tile_C" (Variables|Spawn|GetNextTileTransform) "AdjustIfPossibleButAlwaysSpawn" 0 0))
    (CallFunction|UpdateNextTileTransform _returnvalue)))

(fn ConstructionScript)

(fn GetLastTile'sTransform
  (params (TilesInTheWorld :type Array%20of%20BP%20Tile%20Object%20References))
  (return (Transformation|GetWorldTransform (Variables|/Game/Blueprints/Tiles/BP_Tile.BP_Tile_C|GetAttachPoint (Utilities|Array|Get(acopy) TilesInTheWorld (Utilities|Array|LastIndex TilesInTheWorld))))))

(fn IsThereAnyTileintheWorld
  (params (TilesInTheWorld :type Array%20of%20BP%20Tile%20Object%20References))
  (return (> (Utilities|Array|Length TilesInTheWorld) 0)))

(fn UpdateNextTileTransform
  (params (SpawnedTile :type BP%20Tile%20Object%20Reference))
  (bind _attachlocation (Default|GetAttachPoint SpawnedTile))
  (Variables|Spawn|SetNextTileTransform _attachlocation))