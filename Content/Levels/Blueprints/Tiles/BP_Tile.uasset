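; BP_Tile is a procedural terrain tile with a door and an attach point transform exposed through GetAttachPoint.
; Trigger overlaps by player-tagged actors unlock the door (no collision, translucent green), lock it behind them (solid, red), or destroy the tile.
; Ending overlap with the locking trigger also asks BP_ProceduralTerrainGameMode to spawn another tile, without checking the player tag.
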(event OnComponentBeginOverlap(DoorUnlockingCollision)
  (params (OverlappedComponent :type Primitive%20Component%20Object%20Reference) (OtherActor :type Actor%20Object%20Reference) (OtherComp :type Primitive%20Component%20Object%20Reference) (OtherBodyIndex :type Integer) (bFromSweep :type Boolean) (SweepResult :type Hit%20Result%20Structure%20%28by%20ref%29))
  (Door|DoorUnlock OtherActor))

(event OnComponentEndOverlap(DoorLockingCollision)
  (params (OverlappedComponent :type Primitive%20Component%20Object%20Reference) (OtherActor :type Actor%20Object%20Reference) (OtherComp :type Primitive%20Component%20Object%20Reference) (OtherBodyIndex :type Integer))
  (Door|DoorLock OtherActor)
  (Spawn|SpawnNextTile))

(event OnComponentBeginOverlap(TileDestructionCollision)
  (params (OverlappedComponent :type Primitive%20Component%20Object%20Reference) (OtherActor :type Actor%20Object%20Reference) (OtherComp :type Primitive%20Component%20Object%20Reference) (OtherBodyIndex :type Integer) (bFromSweep :type Boolean) (SweepResult :type Hit%20Result%20Structure%20%28by%20ref%29))
  (Destruction|DestroyTile OtherActor))

(event EventBeginPlay
  (Rendering|Material|SetMaterial (Variables|Default|GetDoor) 0 "/Game/Static/MaterialsPack/Materials/Metal_CyberCube.Metal_CyberCube"))

(fn ConstructionScript)

(fn GetAttachPoint
  (return (Transformation|GetWorldTransform (Variables|Default|GetAttachPoint))))

(fn DoorUnlock
  (params (ActorOverlapping :type Actor%20Object%20Reference))
  (bind _door (Variables|Default|GetDoor))
  (if (Actor|ActorHasTag ActorOverlapping (Utilities|String|StringToName (Variables|Tag|GetPlayerTag)))
    (Collision|SetCollisionEnabled _door "NoCollision")
    (Rendering|Material|SetMaterial _door 0 "/Game/Static/MaterialsPack/Materials/TranslucentGreenMetal_CyberCube.TranslucentGreenMetal_CyberCube")))

(fn DoorLock
  (params (ActorOverlapping :type Actor%20Object%20Reference))
  (bind _door (Variables|Default|GetDoor))
  (if (Actor|ActorHasTag ActorOverlapping (Utilities|String|StringToName (Variables|Tag|GetPlayerTag)))
    (Collision|SetCollisionEnabled _door "QueryAndPhysics")
    (Rendering|Material|SetMaterial _door 0 "/Game/Static/MaterialsPack/Materials/RedMetal_CyberCube.RedMetal_CyberCube")))

(fn SpawnNextTile
  (bind _asbp_procedural_terrain_game_mode (Utilities|Casting|CastToBP_ProceduralTerrainGameMode (Game|GetGameMode)))
  (Default|SpawnTile _asbp_procedural_terrain_game_mode))

(fn DestroyTile
  (params (ActorOverlapping :type Actor%20Object%20Reference))
  (if (Actor|ActorHasTag ActorOverlapping (Utilities|String|StringToName (Variables|Tag|GetPlayerTag)))
    (Actor|DestroyActor)))