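; BP_NPCAI is an NPC AI controller that runs the ChaseAndPatrol behavior tree on the PatrolData blackboard from BeginPlay.
; AI perception updates feed MoveToActorOrPatrol, which reacts only to BP_TPCharacter actors tagged Player.
; A sensed player is written to the FocalPoint blackboard key, and a lost one clears it.
; Both cases stop current movement, leaving the chase or patrol behavior to the tree.
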(event OnTargetPerceptionUpdated(AIPerception)
  (params (Actor :type Actor%20Object%20Reference) (Stimulus :type AI%20Stimulus%20Structure))
  ;[1 1 1] Set focal point or clear it
  (CallFunction|MovetoActororPatrol (.bSuccessfullySensed (Utilities|Struct|BreakAIStimulus Stimulus)) Actor))

(event EventBeginPlay
  ;[1 1 1] Set blackboard and run behavior tree
  (bind _blackboardcomponent (Class|AIController|UseBlackboard "/Game/NPC/AI/Blackboards/PatrolData.PatrolData"))
  (Variables|AI|SetPatrolBlackboard _blackboardcomponent)
  (AI|RunBehaviorTree "/Game/NPC/AI/BehaviorTrees/ChaseAndPatrol.ChaseAndPatrol"))

(fn ConstructionScript)

(fn MovetoActororPatrol
  (params (WasActorSensed :type Boolean) (TargetActor :type Object%20Object%20Reference))
  (bind _patrolblackboard (Variables|AI|GetPatrolBlackboard))
  (bind _focalpoint (Variables|PatrolandChase|GetFocalPoint))
  (bind _returnvalue (Utilities|String|StringToName _focalpoint))
  (bind _asbp_tpcharacter (Utilities|Casting|CastToBP_TPCharacter TargetActor))
  (if (Actor|ActorHasTag _asbp_tpcharacter "Player")
    (if WasActorSensed
      (AI|Components|Blackboard|SetValueasObject _patrolblackboard _returnvalue TargetActor)
      (AI|Navigation|StopMovement)
      (else
        (AI|Components|Blackboard|ClearValue _patrolblackboard _returnvalue)
        (AI|Navigation|StopMovement)))))