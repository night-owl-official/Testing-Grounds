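; NPC AI controller that runs the ChaseAndPatrol behavior tree on the PatrolData blackboard from BeginPlay.
; Perception updates for a TestingGroundsCharacter set it as the FocalPoint blackboard object when sensed and clear that key otherwise.
; Both cases stop current movement, and other actors are ignored.
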(event OnTargetPerceptionUpdated(AIPerception)
  (params (Actor :type Actor%20Object%20Reference) (Stimulus :type AI%20Stimulus%20Structure))
  (CallFunction|MovetoActororPatrol (.bSuccessfullySensed (Utilities|Struct|BreakAIStimulus Stimulus)) Actor))

(event EventBeginPlay
  ;[1 1 1] Set blackboard and run behavior tree
  (bind _blackboardcomponent (Class|AIController|UseBlackboard "/Game/NPC/AI/PatrolData.PatrolData"))
  (Variables|AI|SetPatrolBlackboard _blackboardcomponent)
  (AI|RunBehaviorTree "/Game/NPC/AI/ChaseAndPatrol.ChaseAndPatrol"))

(fn ConstructionScript)

(fn MovetoActororPatrol
  (params (WasActorSensed :type Boolean) (TargetActor :type Object%20Object%20Reference))
  (bind _patrolblackboard (Variables|AI|GetPatrolBlackboard))
  (bind _focalpoint (Variables|PatrolandChase|GetFocalPoint))
  (bind _returnvalue (Utilities|String|StringToName _focalpoint))
  (bind _astesting_grounds_character (Utilities|Casting|CastToTestingGroundsCharacter TargetActor))
  (if WasActorSensed
    (AI|Components|Blackboard|SetValueasObject _patrolblackboard _returnvalue _astesting_grounds_character)
    (AI|Navigation|StopMovement)
    (else
      (AI|Components|Blackboard|ClearValue _patrolblackboard _returnvalue)
      (AI|Navigation|StopMovement))))